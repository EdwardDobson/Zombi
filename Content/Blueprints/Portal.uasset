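; Portal actor that teleports any overlapping actor to a stored exit position, then goes on cooldown.
; Overlap while active moves the actor without sweep, disables the portal and swaps its mesh to a deactivated material.
; Tick counts down a timer while disabled, then re-enables teleporting, resets the timer and restores the portal material.
; The StartTimer function is an empty stub.
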(event `self.ReceiveBeginPlay`)

(event `self.ReceiveActorBeginOverlap`
  (params (OtherActor :type "Actor Object Reference"))
  (if (`self.CanTP`)
    (`self.K2_SetActorLocation` OtherActor (`self.ExitPostion`) false false)
    (set `self.CanTP` false)
    (`PrimitiveComponent.SetMaterial` (`self.StaticMesh`) 0 "/Game/Mats/PortalDeactive.PortalDeactive")))

(event `self.ReceiveTick`
  (params (DeltaSeconds :type "Float (single-precision)"))
  (if (not (`self.CanTP`))
    (bind _output_get (set `self.Timer` (- (`self.Timer`) (`GameplayStatics.GetWorldDeltaSeconds`))))
    (if (< _output_get 0.0)
      (set `self.CanTP` true)
      (set `self.Timer` 3.0)
      (`PrimitiveComponent.SetMaterial` (`self.StaticMesh`) 0 "/Game/Mats/Portal.Portal"))))

(fn `StartTimer`)

(fn `UserConstructionScript`)