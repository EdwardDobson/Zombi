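; Player actor Blueprint with a mouse-aim function and an unwired death check.
; Aim sets actor rotation with zero pitch, using a look-at from the controller's forward vector to a target built from mouse position minus half the viewport size.
; The mouse's vertical coordinate goes into Z, while the viewport's half-height is subtracted from Y.
; Tick is empty, nothing here calls Aim, and the destroy-on-zero-Health logic never runs.
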(event `self.ReceiveTick`
  (params (DeltaSeconds :type "Float (single-precision)")))

(fn `Aim`
  (bind _returnvalue (`GameplayStatics.GetPlayerController` 0))
  (bind (_locationx _locationy) (`PlayerController.GetMousePosition` _returnvalue))
  (`self.K2_SetActorRotation` (`KismetMathLibrary.MakeRotator` (.roll (`KismetMathLibrary.FindLookAtRotation` (`KismetMathLibrary.Conv_RotatorToVector` (`self.K2_GetActorRotation` _returnvalue)) (- (`KismetMathLibrary.MakeVector` _locationx 0.0 _locationy) (`KismetMathLibrary.Conv_Vector2DToVector` (/ (`WidgetLayoutLibrary.GetViewportSize`) 2.0))))) 0.0 (.yaw (`KismetMathLibrary.FindLookAtRotation` (`KismetMathLibrary.Conv_RotatorToVector` (`self.K2_GetActorRotation` _returnvalue)) (- (`KismetMathLibrary.MakeVector` _locationx 0.0 _locationy) (`KismetMathLibrary.Conv_Vector2DToVector` (/ (`WidgetLayoutLibrary.GetViewportSize`) 2.0)))))))
  (return))

(fn `UserConstructionScript`)